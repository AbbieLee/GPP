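; BP_Leverloights is a light actor that signals whether a lever puzzle is in the correct state.
; Its PointLight starts hidden on BeginPlay, turns on through the CorrectLevers event and turns off through IncorrectLevers.
; CorrectLevers also creates a WB_LeverWorked widget, adds it to the viewport and removes it after a short delay.
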(event `self.ReceiveBeginPlay`
  (`SceneComponent.SetVisibility` (`self.PointLight`) false false))

(event `CorrectLevers`
  (bind _wb_leverworked (`self.WB LeverWorked`))
  (`SceneComponent.SetVisibility` (`self.PointLight`) true false)
  (bind _returnvalue (`|CreateWidget` "/Game/Blueprints/UI/Dialogue/WB_LeverWorked.WB_LeverWorked_C"))
  (bind _output_get (set `self.WB LeverWorked` _returnvalue))
  (`UserWidget.AddToViewport` _output_get 0)
  (`KismetSystemLibrary.Delay` 3.0)
  (`/Engine/EditorBlueprintResources/StandardMacros.IsValid` _wb_leverworked
    (:`Is Valid`
      (`Widget.RemoveFromParent` _wb_leverworked))))

(event `IncorrectLevers`
  (`SceneComponent.SetVisibility` (`self.PointLight`) false false))

(fn `UserConstructionScript`)