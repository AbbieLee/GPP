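; Tutorial keypad door that, once opened, runs a timed thaw sequence ending in game over.
; Overlapping the keypad volume enables input, and E toggles the numpad puzzle widget.
; OpenDoor, tied to that puzzle UI, rotates the door via timeline and advances the thaw widget shown after BeginPlay.
; A nested Delay chain swaps thaw stages with ticks, flashes and drips, then disables input, shakes the camera and shows GameOver.
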(event `Open Door`
  (bind _returnvalue (`GameplayStatics.GetPlayerController` 0))
  (bind _returnvalue_2 (`GameplayStatics.GetPlayerController` 0))
  (bind _thaw10b (`self.Thaw10B`))
  (bind _thaw5b (`self.Thaw5B`))
  (bind _thaw0 (`self.Thaw0`))
  (bind _thaw5a (`self.Thaw5A`))
  (bind _thaw10a (`self.Thaw10A`))
  (bind _tick1 (`self.Tick1`))
  (bind _tick2 (`self.Tick2`))
  (bind _tick3 (`self.Tick3`))
  (bind _tick2_2 (`self.Tick2`))
  (bind _tick1_2 (`self.Tick1`))
  (bind _tick1_3 (`self.Tick1`))
  (bind _tick3_2 (`self.Tick3`))
  (bind _thawui (`self.ThawUI`))
  (bind _tick1_4 (`self.Tick1`))
  (bind _thaw40 (`self.Thaw40`))
  (bind _thaw30 (`self.Thaw30`))
  (bind _thaw20 (`self.Thaw20`))
  ; Relation To Puzzle UI Widget
  (`|ExecutionSequence`
    (:`then_0`
      (`GameplayStatics.PlaySound2D` "/Game/Sounds/MetalDoorCreak.MetalDoorCreak" 0.5 0.5 0.0 null null))
    (:`then_1`
      (bind (_direction _opendoorslow) (`Timeline|OpenDoor`)
        (:`Update`
          (`SceneComponent.K2_SetRelativeRotation` (`self.Door`) (`KismetMathLibrary.MakeRotator` 0.0 0.0 (`KismetMathLibrary.Lerp` 0.0 -5.0 _opendoorslow)) false false))))
    (:`then_2`
      (`KismetSystemLibrary.Delay` (`self.TimeInbetween`))
      (`/Engine/EditorBlueprintResources/StandardMacros.IsValid` _thawui
        (:`Is Valid`
          (`Widget.RemoveFromParent` _thawui)
          (`|ExecutionSequence`
            (:`then_0`
              (bind _returnvalue_3 (`|CreateWidget` "/Game/Blueprints/UI/ThawUI/WB_Thaw40.WB_Thaw40_C"))
              (bind _output_get (set `self.Thaw40` _returnvalue_3))
              (`UserWidget.AddToViewport` _output_get -5)
              (`GameplayStatics.PlaySound2D` "/Game/Sounds/TimerTick.TimerTick" 0.2 0.6 0.0 null null)
              (`KismetSystemLibrary.Delay` (`self.TimeInbetween`))
              (`/Engine/EditorBlueprintResources/StandardMacros.IsValid` _thaw40
                (:`Is Valid`
                  (`Widget.RemoveFromParent` _thaw40)
                  (`|ExecutionSequence`
                    (:`then_0`
                      (bind _returnvalue_4 (`|CreateWidget` "/Game/Blueprints/UI/ThawUI/WB_Thaw30.WB_Thaw30_C"))
                      (bind _output_get_2 (set `self.Thaw30` _returnvalue_4))
                      (`UserWidget.AddToViewport` _output_get_2 -5)
                      (`GameplayStatics.PlaySound2D` "/Game/Sounds/TimerTick.TimerTick" 0.2 0.6 0.0 null null)
                      (`KismetSystemLibrary.Delay` (`self.TimeInbetween`))
                      (`/Engine/EditorBlueprintResources/StandardMacros.IsValid` _thaw30
                        (:`Is Valid`
                          (`Widget.RemoveFromParent` _thaw30)
                          (`|ExecutionSequence`
                            (:`then_0`
                              (bind _returnvalue_5 (`|CreateWidget` "/Game/Blueprints/UI/ThawUI/WB_Thaw20.WB_Thaw20_C"))
                              (bind _output_get_3 (set `self.Thaw20` _returnvalue_5))
                              (`UserWidget.AddToViewport` _output_get_3 -5)
                              (`GameplayStatics.PlaySound2D` "/Game/Sounds/TimerTick.TimerTick" 0.2 0.6 0.0 null null)
                              (`KismetSystemLibrary.Delay` (`self.TimeInbetween`))
                              (`/Engine/EditorBlueprintResources/StandardMacros.IsValid` _thaw20
                                (:`Is Valid`
                                  (`Widget.RemoveFromParent` _thaw20)
                                  (`|ExecutionSequence`
                                    (:`then_0`
                                      (bind _returnvalue_6 (`|CreateWidget` "/Game/Blueprints/UI/ThawUI/WB_Thaw10A.WB_Thaw10A_C"))
                                      (bind _output_get_4 (set `self.Thaw10A` _returnvalue_6))
                                      (`UserWidget.AddToViewport` _output_get_4 -5)
                                      (`GameplayStatics.PlaySound2D` "/Game/Sounds/TimerTick.TimerTick" 0.2 0.55 0.0 null null)
                                      (`KismetSystemLibrary.Delay` (`self.TimeInbetween`))
                                      (`/Engine/EditorBlueprintResources/StandardMacros.IsValid` _thaw10a
                                        (:`Is Valid`
                                          (`Widget.RemoveFromParent` _thaw10a)
                                          (`|ExecutionSequence`
                                            (:`then_0`
                                              (bind _returnvalue_7 (`|CreateWidget` "/Game/Blueprints/UI/ThawUI/WB_Thaw5A.WB_Thaw5A_C"))
                                              (bind _output_get_5 (set `self.Thaw5A` _returnvalue_7))
                                              (`UserWidget.AddToViewport` _output_get_5 -5)
                                              (`GameplayStatics.PlaySound2D` "/Game/Sounds/TimerTick.TimerTick" 0.2 0.55 0.0 null null)
                                              (`KismetSystemLibrary.Delay` (`self.TimeInbetween`))
                                              (`/Engine/EditorBlueprintResources/StandardMacros.IsValid` _thaw5a
                                                (:`Is Valid`
                                                  (`Widget.RemoveFromParent` _thaw5a)
                                                  (`|ExecutionSequence`
                                                    (:`then_0`
                                                      (bind _returnvalue_8 (`|CreateWidget` "/Game/Blueprints/UI/ThawUI/WB_Thaw0.WB_Thaw0_C"))
                                                      (bind _output_get_6 (set `self.Thaw0` _returnvalue_8))
                                                      (`UserWidget.AddToViewport` _output_get_6 -5)
                                                      (`GameplayStatics.PlaySound2D` "/Game/Sounds/TimerTick.TimerTick" 0.2 0.5 0.0 null null)
                                                      (`KismetSystemLibrary.Delay` (`self.TimeInbetween`))
                                                      (`/Engine/EditorBlueprintResources/StandardMacros.IsValid` _thaw0
                                                        (:`Is Valid`
                                                          (`Widget.RemoveFromParent` _thaw0)
                                                          (`|ExecutionSequence`
                                                            (:`then_0`
                                                              (bind _returnvalue_9 (`|CreateWidget` "/Game/Blueprints/UI/ThawUI/WB_Thaw5B.WB_Thaw5B_C"))
                                                              (bind _output_get_7 (set `self.Thaw5B` _returnvalue_9))
                                                              (`UserWidget.AddToViewport` _output_get_7 -5)
                                                              (`GameplayStatics.PlaySound2D` "/Game/Sounds/TimerTick.TimerTick" 0.2 0.5 0.0 null null)
                                                              (`KismetSystemLibrary.Delay` (`self.TimeInbetween`))
                                                              (`/Engine/EditorBlueprintResources/StandardMacros.IsValid` _thaw5b
                                                                (:`Is Valid`
                                                                  (`Widget.RemoveFromParent` _thaw5b)
                                                                  (`|ExecutionSequence`
                                                                    (:`then_0`
                                                                      (bind _returnvalue_10 (`|CreateWidget` "/Game/Blueprints/UI/ThawUI/WB_Thaw10B.WB_Thaw10B_C"))
                                                                      (bind _output_get_8 (set `self.Thaw10B` _returnvalue_10))
                                                                      (`UserWidget.AddToViewport` _output_get_8 -5)
                                                                      (`GameplayStatics.PlaySound2D` "/Game/Sounds/TimerTick.TimerTick" 0.3 0.45 0.0 null null)
                                                                      (`KismetSystemLibrary.Delay` 3.0)
                                                                      (`/Engine/EditorBlueprintResources/StandardMacros.IsValid` _thaw10b
                                                                        (:`Is Valid`
                                                                          (`Widget.RemoveFromParent` _thaw10b)
                                                                          (bind _outactors (`GameplayStatics.GetAllActorsOfClass` "/Game/FirstPerson/Blueprints/BP_FirstPersonCharacter.BP_FirstPersonCharacter_C"))
                                                                          (`self.DisableInput` _outactors _returnvalue)
                                                                          (`PlayerController.ClientStartCameraShake` :`self` _returnvalue :`Shake` "/Game/Blueprints/CamShaker.CamShaker_C" :`PlaySpace` "World")
                                                                          (`KismetSystemLibrary.Delay` 0.8)
                                                                          (`|ExecutionSequence`
                                                                            (:`then_0`
                                                                              (bind _returnvalue_11 (`|CreateWidget` "/Game/Blueprints/UI/Menus/WB_GameOver.WB_GameOver_C"))
                                                                              (`UserWidget.AddToViewport` _returnvalue_11 0)
                                                                              (`WidgetBlueprintLibrary.SetInputMode_GameAndUIEx` _returnvalue_2 null)
                                                                              (set `PlayerController.bShowMouseCursor` true _returnvalue_2))
                                                                            (:`then_1`
                                                                              (`GameplayStatics.PlaySound2D` "/Game/Sounds/MonsterGrowl.MonsterGrowl" 1.0 1.0 0.0 null null))))))
                                                                    (:`then_1`
                                                                      (bind _returnvalue_12 (`|CreateWidget` "/Game/Blueprints/UI/ThawUI/WB_FlashingTick1.WB_FlashingTick1_C"))
                                                                      (bind _output_get_9 (set `self.Tick1` _returnvalue_12))
                                                                      (`UserWidget.AddToViewport` _output_get_9 -4)
                                                                      (`|ExecutionSequence`
                                                                        (:`then_0`
                                                                          (`KismetSystemLibrary.Delay` 1.0)
                                                                          (`/Engine/EditorBlueprintResources/StandardMacros.IsValid` _tick1_2
                                                                            (:`Is Valid`
                                                                              (`Widget.RemoveFromParent` _tick1_2))))
                                                                        (:`then_1`
                                                                          (`GameplayStatics.PlaySound2D` "/Game/Sounds/InitialGrowl.InitialGrowl" 1.0 1.0 0.0 null null))))))))
                                                            (:`then_1`
                                                              (bind _returnvalue_13 (`|CreateWidget` "/Game/Blueprints/UI/ThawUI/WB_FlashingTick2.WB_FlashingTick2_C"))
                                                              (bind _output_get_10 (set `self.Tick2` _returnvalue_13))
                                                              (`UserWidget.AddToViewport` _output_get_10 -4)
                                                              (`KismetSystemLibrary.Delay` 1.0)
                                                              (`/Engine/EditorBlueprintResources/StandardMacros.IsValid` _tick2
                                                                (:`Is Valid`
                                                                  (`Widget.RemoveFromParent` _tick2))))
                                                            (:`then_2`
                                                              (`KismetSystemLibrary.Delay` 70.0)
                                                              (`GameplayStatics.PlaySound2D` "/Game/Sounds/DrippingSounds_3.DrippingSounds_3" 0.3 0.9 0.0 null null))))))
                                                    (:`then_1`
                                                      (bind _returnvalue_14 (`|CreateWidget` "/Game/Blueprints/UI/ThawUI/WB_FlashingTick1.WB_FlashingTick1_C"))
                                                      (bind _output_get_11 (set `self.Tick1` _returnvalue_14))
                                                      (`UserWidget.AddToViewport` _output_get_11 -4)
                                                      (`KismetSystemLibrary.Delay` 1.0)
                                                      (`/Engine/EditorBlueprintResources/StandardMacros.IsValid` _tick1_3
                                                        (:`Is Valid`
                                                          (`Widget.RemoveFromParent` _tick1_3))))
                                                    (:`then_2`
                                                      (`KismetSystemLibrary.Delay` 40.0)
                                                      (`GameplayStatics.PlaySound2D` "/Game/Sounds/DrippingSounds_1.DrippingSounds_1" 0.3 0.9 0.0 null null))))))
                                            (:`then_1`
                                              (bind _returnvalue_15 (`|CreateWidget` "/Game/Blueprints/UI/ThawUI/WB_FlashingTick3.WB_FlashingTick3_C"))
                                              (bind _output_get_12 (set `self.Tick3` _returnvalue_15))
                                              (`UserWidget.AddToViewport` _output_get_12 -4)
                                              (`KismetSystemLibrary.Delay` 1.0)
                                              (`/Engine/EditorBlueprintResources/StandardMacros.IsValid` _tick3_2
                                                (:`Is Valid`
                                                  (`Widget.RemoveFromParent` _tick3_2))))))))
                                    (:`then_1`
                                      (bind _returnvalue_16 (`|CreateWidget` "/Game/Blueprints/UI/ThawUI/WB_FlashingTick1.WB_FlashingTick1_C"))
                                      (bind _output_get_13 (set `self.Tick1` _returnvalue_16))
                                      (`UserWidget.AddToViewport` _output_get_13 -4)
                                      (`KismetSystemLibrary.Delay` 1.0)
                                      (`/Engine/EditorBlueprintResources/StandardMacros.IsValid` _tick1
                                        (:`Is Valid`
                                          (`Widget.RemoveFromParent` _tick1))))
                                    (:`then_2`
                                      (`KismetSystemLibrary.Delay` 20.0)
                                      (`GameplayStatics.PlaySound2D` "/Game/Sounds/DrippingSounds_2.DrippingSounds_2" 0.3 0.9 0.0 null null))))))
                            (:`then_1`
                              (bind _returnvalue_17 (`|CreateWidget` "/Game/Blueprints/UI/ThawUI/WB_FlashingTick2.WB_FlashingTick2_C"))
                              (bind _output_get_14 (set `self.Tick2` _returnvalue_17))
                              (`UserWidget.AddToViewport` _output_get_14 -4)
                              (`KismetSystemLibrary.Delay` 1.0)
                              (`/Engine/EditorBlueprintResources/StandardMacros.IsValid` _tick2_2
                                (:`Is Valid`
                                  (`Widget.RemoveFromParent` _tick2_2))))
                            (:`then_2`
                              (`KismetSystemLibrary.Delay` 10.0)
                              (`GameplayStatics.PlaySound2D` "/Game/Sounds/DrippingSounds_3.DrippingSounds_3" 0.3 0.9 0.0 null null))))))
                    (:`then_1`
                      (bind _returnvalue_18 (`|CreateWidget` "/Game/Blueprints/UI/ThawUI/WB_FlashingTick3.WB_FlashingTick3_C"))
                      (bind _output_get_15 (set `self.Tick3` _returnvalue_18))
                      (`UserWidget.AddToViewport` _output_get_15 -4)
                      (`KismetSystemLibrary.Delay` 1.0)
                      (`/Engine/EditorBlueprintResources/StandardMacros.IsValid` _tick3
                        (:`Is Valid`
                          (`Widget.RemoveFromParent` _tick3))))
                    (:`then_2`
                      (`KismetSystemLibrary.Delay` 30.0)
                      (`GameplayStatics.PlaySound2D` "/Game/Sounds/DrippingSounds_1.DrippingSounds_1" 0.3 0.9 0.0 null null))))))
            (:`then_1`
              (bind _returnvalue_19 (`|CreateWidget` "/Game/Blueprints/UI/ThawUI/WB_FlashingTick1.WB_FlashingTick1_C"))
              (bind _output_get_16 (set `self.Tick1` _returnvalue_19))
              (`UserWidget.AddToViewport` _output_get_16 -4)
              (`KismetSystemLibrary.Delay` 1.0)
              (`/Engine/EditorBlueprintResources/StandardMacros.IsValid` _tick1_4
                (:`Is Valid`
                  (`Widget.RemoveFromParent` _tick1_4))))))))
    (:`then_3`
      (`KismetSystemLibrary.Delay` 3.0)
      (`GameplayStatics.PlaySound2D` "/Game/Sounds/DrippingSounds_1.DrippingSounds_1" 0.3 0.9 0.0 null null))))

(event `self.PlayerNearKeypad.OnComponentBeginOverlap`
  (params (OverlappedComponent :type "PrimitiveComponent Object Reference") (OtherActor :type "Actor Object Reference") (OtherComp :type "PrimitiveComponent Object Reference") (OtherBodyIndex :type Integer) (bFromSweep :type Boolean) (SweepResult :type "HitResult Structure (by ref)"))
  ; Allow/Disables Player Input (E)
  (cast `/Game/FirstPerson/Blueprints/BP_FirstPersonCharacter` OtherActor)
  (`self.EnableInput` (`GameplayStatics.GetPlayerController` 0)))

(event `self.PlayerNearKeypad.OnComponentEndOverlap`
  (params (OverlappedComponent :type "PrimitiveComponent Object Reference") (OtherActor :type "Actor Object Reference") (OtherComp :type "PrimitiveComponent Object Reference") (OtherBodyIndex :type Integer))
  (bind _returnvalue (`GameplayStatics.GetPlayerController` 0))
  (bind _numpad (`self.NumPad`))
  ; Allow/Disables Player Input (E)
  (cast `/Game/FirstPerson/Blueprints/BP_FirstPersonCharacter` OtherActor)
  (`self.DisableInput` (`GameplayStatics.GetPlayerController` 0))
  ; Player Input Creates UI Puzzle
  (`/Engine/EditorBlueprintResources/StandardMacros.IsValid` _numpad :!label _label
    (:`Is Valid`
      (`Widget.RemoveFromParent` _numpad)
      (`WidgetBlueprintLibrary.SetInputMode_GameOnly` _returnvalue)
      (set `PlayerController.bShowMouseCursor` false _returnvalue))))

(event `Key|E`
  (params (Key :type "Key Structure"))
  (bind _returnvalue (`GameplayStatics.GetPlayerController` 0))
  ; Player Input Creates UI Puzzle
  (:`Pressed`
    (`/Engine/EditorBlueprintResources/StandardMacros.FlipFlop`
      (:`A`
        (bind _returnvalue_2 (`|CreateWidget` "/Game/Blueprints/UI/WB_TutNumPad.WB_TutNumPad_C"))
        (bind _output_get (set `self.NumPad` _returnvalue_2))
        (`UserWidget.AddToViewport` _output_get 0)
        (`WidgetBlueprintLibrary.SetInputMode_GameAndUIEx` _returnvalue null)
        (set `PlayerController.bShowMouseCursor` true _returnvalue))
      (:`B`
        (goto _label)))))

(event `self.ReceiveBeginPlay`
  ; Initial Sounds & UI
  (`|ExecutionSequence`
    (:`then_0`
      (`KismetSystemLibrary.Delay` 8.0)
      (bind _returnvalue (`|CreateWidget` "/Game/Blueprints/UI/ThawUI/WB_Thaw50.WB_Thaw50_C"))
      (bind _output_get (set `self.ThawUI` _returnvalue))
      (`UserWidget.AddToViewport` _output_get -5))
    (:`then_1`
      (`KismetSystemLibrary.Delay` 20.0)
      (`GameplayStatics.PlaySound2D` "/Game/Sounds/DrippingSounds_3.DrippingSounds_3" 0.3 0.9 0.0 null null))))

(fn `UserConstructionScript`)