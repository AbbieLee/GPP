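; BP_ExitDoor is the game's exit door, which accepts the E key once the first-person character has overlapped its box; the input-disabling branch is unwired.
; Each CogCorrect event appends "1" to a string that must match CorrectA.
; A match triggers a one-time ending of creak sound, stopped breeze audio, fade, cutscene, then continue button and cursor.
; A mismatch briefly shows a failure dialogue widget.
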(event `self.Box.OnComponentBeginOverlap`
  (params (OverlappedComponent :type "PrimitiveComponent Object Reference") (OtherActor :type "Actor Object Reference") (OtherComp :type "PrimitiveComponent Object Reference") (OtherBodyIndex :type Integer) (bFromSweep :type Boolean) (SweepResult :type "HitResult Structure (by ref)"))
  (cast `/Game/FirstPerson/Blueprints/BP_FirstPersonCharacter` OtherActor)
  (`self.EnableInput` (`GameplayStatics.GetPlayerController` 0)))

(event `Key|E`
  (params (Key :type "Key Structure"))
  (bind _dialogue4 (`self.Dialogue4`))
  ; Player Input
  (:`Pressed`
    (if (`KismetStringLibrary.EqualEqual_StrStr` (`self.Value A`) (`self.Correct A`))
      (`/Engine/EditorBlueprintResources/StandardMacros.DoOnce` false
        (:`Completed`
          (`|ExecutionSequence`
            (:`then_0`
              (`KismetSystemLibrary.Delay` 2.5)
              (`AudioComponent.Stop` (`self.IndoorBreeze`)))
            (:`then_1`
              (bind _returnvalue (`|CreateWidget` "/Game/Blueprints/UI/Menus/WB_FadeToBlack.WB_FadeToBlack_C"))
              (`UserWidget.AddToViewport` _returnvalue 0)
              (`KismetSystemLibrary.Delay` 3.0)
              (`|ExecutionSequence`
                (:`then_0`
                  (`GameplayStatics.PlaySound2D` "/Game/Sounds/2__Ending_Cutscene.2__Ending_Cutscene" 1.0 1.0 0.0 null null))
                (:`then_1`
                  (bind _returnvalue_2 (`|CreateWidget` "/Game/Blueprints/UI/Menus/WB_Custscene2.WB_Custscene2_C"))
                  (`UserWidget.AddToViewport` _returnvalue_2 0)
                  (`KismetSystemLibrary.Delay` 12.0)
                  (`|ExecutionSequence`
                    (:`then_0`
                      (bind _returnvalue_3 (`|CreateWidget` "/Game/Blueprints/UI/Menus/WB_ContinueButton2.WB_ContinueButton2_C"))
                      (`UserWidget.AddToViewport` _returnvalue_3 0))
                    (:`then_1`
                      (set `PlayerController.bShowMouseCursor` true (`GameplayStatics.GetPlayerController` 0)))))))
            (:`then_2`
              (`GameplayStatics.PlaySound2D` "/Game/Sounds/MetalDoorCreak.MetalDoorCreak" 1.0 1.0 0.0 null null)))))
      (else
        ; Didn't Work Dialogue
        (bind _returnvalue_4 (`|CreateWidget` "/Game/Blueprints/UI/Dialogue/WB_Dialogue4ExitNOwork.WB_Dialogue4ExitNOwork_C"))
        (bind _output_get (set `self.Dialogue4` _returnvalue_4))
        (`UserWidget.AddToViewport` _output_get 0)
        (`KismetSystemLibrary.Delay` 4.0)
        (`/Engine/EditorBlueprintResources/StandardMacros.IsValid` _dialogue4
          (:`Is Valid`
            (`Widget.RemoveFromParent` _dialogue4)))))))

(event `CogCorrect`
  ; Cog Placement Sets Value
  (set `self.Value A` (`KismetStringLibrary.Concat_StrStr` (`self.Value A`) "1")))

(event `self.ReceiveBeginPlay`
  (bind _returnvalue (`AddComponent|NODE_AddAudioComponent-0`))
  (set `self.IndoorBreeze` _returnvalue))

(fn `Get Name`
  (returns (Name :type Text))
  (return (`self.Name`)))

(fn `UserConstructionScript`)