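; BP_ThawTimer drives an on-screen thaw indicator that steps through a fixed series of stage widgets at one-minute intervals.
; The ThawTimer event chains latent Delays, each removing the current widget if valid and creating the next, mostly at a negative Z-order.
; Widget names count down from Thaw50 to Thaw0, then continue through Thaw5B and Thaw10B before the last is removed.
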(event `ThawTimer`
  (bind _thaw10b (`self.Thaw10B`))
  (bind _thaw5b (`self.Thaw5B`))
  (bind _thaw0 (`self.Thaw0`))
  (bind _thaw5a (`self.Thaw5A`))
  (bind _thaw10a (`self.Thaw10A`))
  (bind _thawui (`self.ThawUI`))
  (bind _thaw40 (`self.Thaw40`))
  (bind _thaw30 (`self.Thaw30`))
  (bind _thaw20 (`self.Thaw20`))
  (bind _returnvalue (`|CreateWidget` "/Game/Blueprints/UI/ThawUI/WB_Thaw50.WB_Thaw50_C"))
  (bind _output_get (set `self.ThawUI` _returnvalue))
  (`UserWidget.AddToViewport` _output_get 0)
  (`KismetSystemLibrary.Delay` 60.0)
  (`/Engine/EditorBlueprintResources/StandardMacros.IsValid` _thawui
    (:`Is Valid`
      (`Widget.RemoveFromParent` _thawui)
      (bind _returnvalue_2 (`|CreateWidget` "/Game/Blueprints/UI/ThawUI/WB_Thaw40.WB_Thaw40_C"))
      (bind _output_get_2 (set `self.Thaw40` _returnvalue_2))
      (`UserWidget.AddToViewport` _output_get_2 -5)
      (`KismetSystemLibrary.Delay` 60.0)
      (`/Engine/EditorBlueprintResources/StandardMacros.IsValid` _thaw40
        (:`Is Valid`
          (`Widget.RemoveFromParent` _thaw40)
          (bind _returnvalue_3 (`|CreateWidget` "/Game/Blueprints/UI/ThawUI/WB_Thaw30.WB_Thaw30_C"))
          (bind _output_get_3 (set `self.Thaw30` _returnvalue_3))
          (`UserWidget.AddToViewport` _output_get_3 -5)
          (`KismetSystemLibrary.Delay` 60.0)
          (`/Engine/EditorBlueprintResources/StandardMacros.IsValid` _thaw30
            (:`Is Valid`
              (`Widget.RemoveFromParent` _thaw30)
              (bind _returnvalue_4 (`|CreateWidget` "/Game/Blueprints/UI/ThawUI/WB_Thaw20.WB_Thaw20_C"))
              (bind _output_get_4 (set `self.Thaw20` _returnvalue_4))
              (`UserWidget.AddToViewport` _output_get_4 -5)
              (`KismetSystemLibrary.Delay` 60.0)
              (`/Engine/EditorBlueprintResources/StandardMacros.IsValid` _thaw20
                (:`Is Valid`
                  (`Widget.RemoveFromParent` _thaw20)
                  (bind _returnvalue_5 (`|CreateWidget` "/Game/Blueprints/UI/ThawUI/WB_Thaw10A.WB_Thaw10A_C"))
                  (bind _output_get_5 (set `self.Thaw10A` _returnvalue_5))
                  (`UserWidget.AddToViewport` _output_get_5 -5)
                  (`KismetSystemLibrary.Delay` 60.0)
                  (`/Engine/EditorBlueprintResources/StandardMacros.IsValid` _thaw10a
                    (:`Is Valid`
                      (`Widget.RemoveFromParent` _thaw10a)
                      (bind _returnvalue_6 (`|CreateWidget` "/Game/Blueprints/UI/ThawUI/WB_Thaw5A.WB_Thaw5A_C"))
                      (bind _output_get_6 (set `self.Thaw5A` _returnvalue_6))
                      (`UserWidget.AddToViewport` _output_get_6 -5)
                      (`KismetSystemLibrary.Delay` 60.0)
                      (`/Engine/EditorBlueprintResources/StandardMacros.IsValid` _thaw5a
                        (:`Is Valid`
                          (`Widget.RemoveFromParent` _thaw5a)
                          (bind _returnvalue_7 (`|CreateWidget` "/Game/Blueprints/UI/ThawUI/WB_Thaw0.WB_Thaw0_C"))
                          (bind _output_get_7 (set `self.Thaw0` _returnvalue_7))
                          (`UserWidget.AddToViewport` _output_get_7 -5)
                          (`KismetSystemLibrary.Delay` 60.0)
                          (`/Engine/EditorBlueprintResources/StandardMacros.IsValid` _thaw0
                            (:`Is Valid`
                              (`Widget.RemoveFromParent` _thaw0)
                              (bind _returnvalue_8 (`|CreateWidget` "/Game/Blueprints/UI/ThawUI/WB_Thaw5B.WB_Thaw5B_C"))
                              (bind _output_get_8 (set `self.Thaw5B` _returnvalue_8))
                              (`UserWidget.AddToViewport` _output_get_8 -5)
                              (`KismetSystemLibrary.Delay` 60.0)
                              (`/Engine/EditorBlueprintResources/StandardMacros.IsValid` _thaw5b
                                (:`Is Valid`
                                  (`Widget.RemoveFromParent` _thaw5b)
                                  (bind _returnvalue_9 (`|CreateWidget` "/Game/Blueprints/UI/ThawUI/WB_Thaw10B.WB_Thaw10B_C"))
                                  (bind _output_get_9 (set `self.Thaw10B` _returnvalue_9))
                                  (`UserWidget.AddToViewport` _output_get_9 -5)
                                  (`KismetSystemLibrary.Delay` 60.0)
                                  (`/Engine/EditorBlueprintResources/StandardMacros.IsValid` _thaw10b
                                    (:`Is Valid`
                                      (`Widget.RemoveFromParent` _thaw10b))))))))))))))))))))

(fn `UserConstructionScript`)