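; BP_OrganPuzzleDrawer is a drawer that slides open when the organ jar puzzle is solved.
; Its JarsSorted event plays the OpenDraw timeline, which drives the Drawer component's relative location.
; Each timeline update also creates a WB_OrganPuzzleWorked widget, adds it to the viewport and overwrites the stored reference.
; A nine-second delay then removes only the referenced widget.
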(event `self.ReceiveBeginPlay`)

(event `self.ReceiveTick`
  (params (DeltaSeconds :type "Float (single-precision)")))

(event `JarsSorted`
  (bind _opuzzleworked (`self.OPuzzleWorked`))
  (bind (_direction _newtrack_0) (`Timeline|OpenDraw`)
    (:`Update`
      (`SceneComponent.K2_SetRelativeLocation` (`self.Drawer`) _newtrack_0 false false)
      (bind _returnvalue (`|CreateWidget` "/Game/Blueprints/UI/Dialogue/WB_OrganPuzzleWorked.WB_OrganPuzzleWorked_C"))
      (bind _output_get (set `self.OPuzzleWorked` _returnvalue))
      (`UserWidget.AddToViewport` _output_get 0)
      (`KismetSystemLibrary.Delay` 9.0)
      (`/Engine/EditorBlueprintResources/StandardMacros.IsValid` _opuzzleworked
        (:`Is Valid`
          (`Widget.RemoveFromParent` _opuzzleworked))))))

(fn `Get Name`
  (returns (Name :type Text))
  (return (`self.Name`)))

(fn `UserConstructionScript`)