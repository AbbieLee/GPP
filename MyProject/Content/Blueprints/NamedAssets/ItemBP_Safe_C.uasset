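; Interactable safe Blueprint that presents a combination-lock puzzle and plays an opening sequence when unlocked.
; An overlap volume enables E input for the first-person character; E flip-flops the WB_CombiLock widget, cursor and input mode, and leaving the area closes it.
; UnlockedSafe runs chained timelines for the dropping padlock, lock and door rotation, alongside a revealed point light and delayed sounds.
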(event `Unlocked Safe`
  (`|ExecutionSequence`
    (:`then_0`
      ; Lock Anim
      (bind (_direction _lockdrop) (`Timeline|LockDrop`)
        (:`Update`
          (`SceneComponent.K2_SetRelativeLocation` (`self.Lock`) _lockdrop false false)
          (bind (_direction_2 _fallroat) (`Timeline|LockRotation`)
            (:`Update`
              (`SceneComponent.K2_SetRelativeRotation` (`self.Lock`) (`KismetMathLibrary.MakeRotator` (`KismetMathLibrary.Lerp` 0.0 5.0 _fallroat)) false false))))))
    (:`then_1`
      ; Safe Door Anim
      (`KismetSystemLibrary.Delay` 1.0)
      (bind (_direction_3 _safelokc) (`Timeline|SafeLockOpening`)
        (:`Update`
          (`SceneComponent.K2_SetRelativeRotation` (`self.Abbie_-_SafeLock`) (`KismetMathLibrary.MakeRotator` 0.0 0.0 (`KismetMathLibrary.Lerp` 0.0 5.0 _safelokc)) false false))
        (:`Finished`
          (bind (_direction_4 _opendoor) (`Timeline|SafeDoorOpening`)
            (:`Update`
              (`SceneComponent.K2_SetRelativeRotation` (`self.Abbie_-_SafeDoor`) (`KismetMathLibrary.MakeRotator` 0.0 0.0 (`KismetMathLibrary.Lerp` 0.0 -5.0 _opendoor)) false false))))))
    (:`then_2`
      (`SceneComponent.SetVisibility` (`self.PointLight`) true false))
    (:`then_3`
      (`KismetSystemLibrary.Delay` 1.5)
      (`GameplayStatics.PlaySound2D` "/Game/Sounds/SafeDooropening.SafeDooropening" 1.0 1.0 0.0 null null)
      (`KismetSystemLibrary.Delay` 1.5)
      (`GameplayStatics.PlaySound2D` "/Game/Sounds/LightOnLonger.LightOnLonger" 1.0 1.0 0.0 null null))))

(event `self.ReceiveBeginPlay`
  (`SceneComponent.SetVisibility` (`self.PointLight`) false false))

(event `self.In Area.OnComponentBeginOverlap`
  (params (OverlappedComponent :type "PrimitiveComponent Object Reference") (OtherActor :type "Actor Object Reference") (OtherComp :type "PrimitiveComponent Object Reference") (OtherBodyIndex :type Integer) (bFromSweep :type Boolean) (SweepResult :type "HitResult Structure (by ref)"))
  ; Allow/Disables Player Input (E)
  (cast `/Game/FirstPerson/Blueprints/BP_FirstPersonCharacter` OtherActor)
  (`self.EnableInput` (`GameplayStatics.GetPlayerController` 0)))

(event `self.In Area.OnComponentEndOverlap`
  (params (OverlappedComponent :type "PrimitiveComponent Object Reference") (OtherActor :type "Actor Object Reference") (OtherComp :type "PrimitiveComponent Object Reference") (OtherBodyIndex :type Integer))
  (bind _returnvalue (`GameplayStatics.GetPlayerController` 0))
  (bind _wb_scroll_ (`self.WB Scroll `))
  ; Allow/Disables Player Input (E)
  (cast `/Game/FirstPerson/Blueprints/BP_FirstPersonCharacter` OtherActor)
  (`self.DisableInput` (`GameplayStatics.GetPlayerController` 0))
  ; Player Input Creates UI Puzzle
  (`/Engine/EditorBlueprintResources/StandardMacros.IsValid` _wb_scroll_ :!label _label
    (:`Is Valid`
      (`Widget.RemoveFromParent` _wb_scroll_)
      (`WidgetBlueprintLibrary.SetInputMode_GameOnly` _returnvalue)
      (set `PlayerController.bShowMouseCursor` false _returnvalue))))

(event `Key|E`
  (params (Key :type "Key Structure"))
  (bind _returnvalue (`GameplayStatics.GetPlayerController` 0))
  ; Player Input Creates UI Puzzle
  (:`Pressed`
    (`/Engine/EditorBlueprintResources/StandardMacros.FlipFlop`
      (:`A`
        (bind _returnvalue_2 (`|CreateWidget` "/Game/Blueprints/UI/WB_CombiLock.WB_CombiLock_C"))
        (bind _output_get (set `self.WB Scroll ` _returnvalue_2))
        (`UserWidget.AddToViewport` _output_get 0)
        (`WidgetBlueprintLibrary.SetInputMode_GameAndUIEx` _returnvalue null)
        (set `PlayerController.bShowMouseCursor` true _returnvalue))
      (:`B`
        (goto _label)))))

(fn `UserConstructionScript`
  (`parent.UserConstructionScript`))