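; Lever puzzle item with four levers whose roll angles form a code that drives a linked lights actor.
; Interacting rotates a lever by a fixed step up or down and plays a sound; BeginPlay offsets the first and third levers.
; Each move marks that lever correct if its roll nearly matches either of two code arrays.
; The lights actor then shows correct, with a sound, only if all entries pass, otherwise incorrect.
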(event `/Game/Blueprints/InteractWithLevers.Interact With Levers`
  (params (Component :type "PrimitiveComponent Object Reference") (LeverUp :type Boolean))
  (`self.Rotation` Component LeverUp)
  (`GameplayStatics.PlaySound2D` "/Game/Sounds/Lever.Lever" 1.0 1.0 0.0 null null))

(event `self.ReceiveBeginPlay`
  (`self.Initial Rotation` (`self.L1`))
  (`self.Initial Rotation` (`self.L3`)))

(fn `Check Code`
  (params (Component :type "PrimitiveComponent Object Reference"))
  (locals (`Selected Mesh` :type Integer) (`Local Fail` :type Boolean :default false))
  (bind _leverlights (`self.Leverlights`))
  (bind _relativerotation_roll (`KismetMathLibrary.BreakRotator` (`SceneComponent.RelativeRotation` Component)))
  (bind _relativerotation_roll_2 (`KismetMathLibrary.BreakRotator` (`SceneComponent.RelativeRotation` Component)))
  ; Lever Inputs
  (if (== Component (`self.L1`))
    (set `local.Selected Mesh` 0)
    (`KismetArrayLibrary.Array_Set` (`self.CorrectCode`) (`local.Selected Mesh`) (or (`KismetMathLibrary.NearlyEqual_FloatFloat` (`|GetArrayItem` (`self.Code2`) (`local.Selected Mesh`)) _relativerotation_roll_2 5.0) (`KismetMathLibrary.NearlyEqual_FloatFloat` (`|GetArrayItem` (`self.Code`) (`local.Selected Mesh`)) _relativerotation_roll 5.0)) :!label _label)
    (for _array_element (`self.CorrectCode`)
      (if (not _array_element)
        (set `local.Local Fail` true)
        (break)))
    (if (`local.Local Fail`)
      (`/Engine/EditorBlueprintResources/StandardMacros.IsValid` _leverlights
        (:`Is Valid`
          (`/Game/Blueprints/BP_Leverloights.IncorrectLevers` _leverlights)))
      (else
        (`/Engine/EditorBlueprintResources/StandardMacros.IsValid` _leverlights
          (:`Is Valid`
            (`/Game/Blueprints/BP_Leverloights.CorrectLevers` _leverlights)
            (`GameplayStatics.PlaySound2D` "/Game/Sounds/LightOn.LightOn" 1.0 1.0 0.0 null null)))))
    (elif (== Component (`self.L2`))
      (set `local.Selected Mesh` 1)
      (goto _label)
      (elif (== Component (`self.L3`))
        (set `local.Selected Mesh` 2)
        (goto _label)
        (elif (== Component (`self.L4`))
          (set `local.Selected Mesh` 3)
          (goto _label))))))

(fn `Initial Rotation`
  (params (Component :type "PrimitiveComponent Object Reference") (Up :type Boolean))
  (if Up
    (`SceneComponent.K2_AddRelativeRotation` Component (`KismetMathLibrary.MakeRotator` (`self.Start Value`)) false false)
    (`KismetSystemLibrary.PrintString` (`KismetStringLibrary.Conv_RotatorToString` (`SceneComponent.RelativeRotation` Component)))
    (else
      (`SceneComponent.K2_AddRelativeRotation` Component (`KismetMathLibrary.MakeRotator` (* (`self.Start Value`) -1.0)) false false)))
  (`self.Check Code` Component))

(fn `Rotation`
  (params (Component :type "PrimitiveComponent Object Reference") (Up :type Boolean))
  (if Up
    (`SceneComponent.K2_AddRelativeRotation` Component (`KismetMathLibrary.MakeRotator` (`self.Rotation Value`)) false false)
    (else
      (`SceneComponent.K2_AddRelativeRotation` Component (`KismetMathLibrary.MakeRotator` (* (`self.Rotation Value`) -1.0)) false false)))
  (`self.Check Code` Component))

(fn `UserConstructionScript`
  (`parent.UserConstructionScript`))