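; Journal entry item that the player can read as an on-screen note once its safe is unlocked.
; Box overlap with the first-person character toggles input, and UnlockedSafeSetBool sets the flag that gates the Q key.
; A FlipFlop on Q alternates between opening the levers note widget with a paper sound and mouse cursor, and closing it.
; Leaving the box also closes the note and restores game-only input.
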(event `self.ReceiveBeginPlay`
  (`parent.ReceiveBeginPlay`)
  (set `self.SafeUnlocked` false))

(event `self.Box.OnComponentBeginOverlap`
  (params (OverlappedComponent :type "PrimitiveComponent Object Reference") (OtherActor :type "Actor Object Reference") (OtherComp :type "PrimitiveComponent Object Reference") (OtherBodyIndex :type Integer) (bFromSweep :type Boolean) (SweepResult :type "HitResult Structure (by ref)"))
  (cast `/Game/FirstPerson/Blueprints/BP_FirstPersonCharacter` OtherActor)
  (`self.EnableInput` (`GameplayStatics.GetPlayerController` 0)))

(event `self.Box.OnComponentEndOverlap`
  (params (OverlappedComponent :type "PrimitiveComponent Object Reference") (OtherActor :type "Actor Object Reference") (OtherComp :type "PrimitiveComponent Object Reference") (OtherBodyIndex :type Integer))
  (bind _returnvalue (`GameplayStatics.GetPlayerController` 0))
  (bind _wb_note_inspection_2 (`self.WB Note Inspection 2`))
  (cast `/Game/FirstPerson/Blueprints/BP_FirstPersonCharacter` OtherActor)
  (`self.DisableInput` (`GameplayStatics.GetPlayerController` 0))
  ; Player Input Creates UI Puzzle
  (`/Engine/EditorBlueprintResources/StandardMacros.IsValid` _wb_note_inspection_2 :!label _label
    (:`Is Valid`
      (`Widget.RemoveFromParent` _wb_note_inspection_2)
      (`WidgetBlueprintLibrary.SetInputMode_GameOnly` _returnvalue)
      (set `PlayerController.bShowMouseCursor` false _returnvalue))))

(event `Key|Q`
  (params (Key :type "Key Structure"))
  (bind _returnvalue (`GameplayStatics.GetPlayerController` 0))
  (:`Pressed`
    ; Player Input Creates UI Puzzle
    (if (`self.SafeUnlocked`)
      (`/Engine/EditorBlueprintResources/StandardMacros.FlipFlop`
        (:`A`
          (`|ExecutionSequence`
            (:`then_0`
              (`GameplayStatics.PlaySound2D` "/Game/Sounds/PaperPickup.PaperPickup" 1.0 1.0 0.0 null null))
            (:`then_1`
              (bind _returnvalue_2 (`|CreateWidget` "/Game/Blueprints/UI/Screens/WB_NoteInsp_Levers.WB_NoteInsp_Levers_C"))
              (bind _output_get (set `self.WB Note Inspection 2` _returnvalue_2))
              (`UserWidget.AddToViewport` _output_get 0)
              (`WidgetBlueprintLibrary.SetInputMode_GameAndUIEx` _returnvalue null)
              (set `PlayerController.bShowMouseCursor` true _returnvalue))))
        (:`B`
          (goto _label))))))

(event `UnlockedSafeSetBool`
  ; Sets Unlocked Safe Bool = True
  (set `self.SafeUnlocked` true))

(fn `UserConstructionScript`
  (`parent.UserConstructionScript`))