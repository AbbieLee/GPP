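; Jar placement spot actor where a jar can be spawned into the world.
; An overlap box enables the actor's input while the first-person character is inside and disables it on exit.
; The PlaceJar event spawns a scaled-down ItemBP_Jar1 at the JarPlace1 component's world location, with no check on inventory or earlier placement.
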(event `self.Box.OnComponentBeginOverlap`
  (params (OverlappedComponent :type "PrimitiveComponent Object Reference") (OtherActor :type "Actor Object Reference") (OtherComp :type "PrimitiveComponent Object Reference") (OtherBodyIndex :type Integer) (bFromSweep :type Boolean) (SweepResult :type "HitResult Structure (by ref)"))
  (cast `/Game/FirstPerson/Blueprints/BP_FirstPersonCharacter` OtherActor)
  (`self.EnableInput` (`GameplayStatics.GetPlayerController` 0)))

(event `self.Box.OnComponentEndOverlap`
  (params (OverlappedComponent :type "PrimitiveComponent Object Reference") (OtherActor :type "Actor Object Reference") (OtherComp :type "PrimitiveComponent Object Reference") (OtherBodyIndex :type Integer))
  (cast `/Game/FirstPerson/Blueprints/BP_FirstPersonCharacter` OtherActor)
  (`self.DisableInput` (`GameplayStatics.GetPlayerController` 0)))

(event `/Game/Blueprints/BPI_PlaceJar.PlaceJar`
  (params (component :type "PrimitiveComponent Object Reference"))
  (`|SpawnActorFromClass` "/Game/Blueprints/NamedAssets/ItemBP_Jar1_C.ItemBP_Jar1_C_C" (`KismetMathLibrary.MakeTransform` (`SceneComponent.K2_GetComponentLocation` (`self.JarPlace1`)) (struct) (0.2 0.2 0.2)) "Undefined" "MultiplyWithRoot" null null))

(fn `UserConstructionScript`
  (`parent.UserConstructionScript`))