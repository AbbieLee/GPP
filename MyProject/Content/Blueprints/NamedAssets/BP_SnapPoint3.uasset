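; BP_SnapPoint3 is a snap point where the player places a cog to progress toward the exit door.
; Its mesh hides at BeginPlay and appears when a component with the matching tag overlaps the box, which destroys that component.
; It then destroys the cog item, calls CogCorrect on the exit door and plays a click.
; A temporary dialogue widget and a one-time voice clip follow.
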(event `self.ReceiveBeginPlay`
  (`SceneComponent.SetVisibility` (`self.StaticMesh`) false false))

(event `self.Box.OnComponentBeginOverlap`
  (params (OverlappedComponent :type "PrimitiveComponent Object Reference") (OtherActor :type "Actor Object Reference") (OtherComp :type "PrimitiveComponent Object Reference") (OtherBodyIndex :type Integer) (bFromSweep :type Boolean) (SweepResult :type "HitResult Structure (by ref)"))
  (bind _dialogue5 (`self.Dialogue5`))
  (if (`ActorComponent.ComponentHasTag` OtherComp (`self.Tag`))
    (`ActorComponent.K2_DestroyComponent` OtherComp)
    (`SceneComponent.SetVisibility` (`self.StaticMesh`) true false)
    (`|ExecutionSequence`
      (:`then_0`
        (bind _returnvalue (`GameplayStatics.GetActorOfClass` "/Game/Blueprints/NamedAssets/ItemBP_Cog_C.ItemBP_Cog_C_C"))
        (`/Game/Blueprints/NamedAssets/ItemBP_Cog_C.DestroyItem` _returnvalue))
      (:`then_1`
        (bind _returnvalue_2 (`GameplayStatics.GetActorOfClass` "/Game/Blueprints/BP_ExitDoor.BP_ExitDoor_C"))
        (`/Game/Blueprints/BP_ExitDoor.CogCorrect` _returnvalue_2)
        (`GameplayStatics.PlaySound2D` "/Game/Sounds/SwitchClick.SwitchClick" 1.0 1.0 0.0 null null))
      (:`then_2`
        (bind _returnvalue_3 (`|CreateWidget` "/Game/Blueprints/UI/Dialogue/WB_Dialogue5CogPlaced.WB_Dialogue5CogPlaced_C"))
        (bind _output_get (set `self.Dialogue5` _returnvalue_3))
        (`UserWidget.AddToViewport` _output_get 0)
        (`KismetSystemLibrary.Delay` 4.0)
        (`/Engine/EditorBlueprintResources/StandardMacros.IsValid` _dialogue5
          (:`Is Valid`
            (`Widget.RemoveFromParent` _dialogue5))))
      (:`then_3`
        (`/Engine/EditorBlueprintResources/StandardMacros.DoOnce` false
          (:`Completed`
            (`GameplayStatics.PlaySound2D` "/Game/Sounds/FinalVoiceLines/10__Finally.10__Finally" 1.0 1.0 0.0 null null)))))))

(fn `UserConstructionScript`)