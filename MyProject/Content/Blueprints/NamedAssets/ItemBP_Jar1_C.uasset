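; Jar item Blueprint that the first-person character can pick up.
; A Box overlap enables input on the jar for player 0 while that character is inside and disables it on exit.
; PickUp returns the BaseAsset static mesh to the caller and calls DestroyItem, which removes the actor after a short delay.
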(event `DestroyItem`
  (`KismetSystemLibrary.Delay` 0.2)
  (`self.K2_DestroyActor`))

(event `self.Box.OnComponentBeginOverlap`
  (params (OverlappedComponent :type "PrimitiveComponent Object Reference") (OtherActor :type "Actor Object Reference") (OtherComp :type "PrimitiveComponent Object Reference") (OtherBodyIndex :type Integer) (bFromSweep :type Boolean) (SweepResult :type "HitResult Structure (by ref)"))
  (cast `/Game/FirstPerson/Blueprints/BP_FirstPersonCharacter` OtherActor)
  (`self.EnableInput` (`GameplayStatics.GetPlayerController` 0)))

(event `self.Box.OnComponentEndOverlap`
  (params (OverlappedComponent :type "PrimitiveComponent Object Reference") (OtherActor :type "Actor Object Reference") (OtherComp :type "PrimitiveComponent Object Reference") (OtherBodyIndex :type Integer))
  (cast `/Game/FirstPerson/Blueprints/BP_FirstPersonCharacter` OtherActor)
  (`self.DisableInput` (`GameplayStatics.GetPlayerController` 0)))

(fn `PickUp`
  (params (Component :type "PrimitiveComponent Object Reference"))
  (returns (`Static Mesh` :type "StaticMesh Object Reference"))
  (`self.DestroyItem`)
  (return (`StaticMeshComponent.StaticMesh` (`self.Base Asset`))))

(fn `UserConstructionScript`
  (`parent.UserConstructionScript`))