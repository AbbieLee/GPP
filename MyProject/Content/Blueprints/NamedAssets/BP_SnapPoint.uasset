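; BP_SnapPoint is a snap target for placing Jar 1 in the organ drawer puzzle.
; Its static mesh starts hidden and is revealed when a component with the matching tag overlaps the Box, destroying that component to fake the snap.
; It then calls DestroyItem on the ItemBP_Jar1 actors and SetValJarA on the BP_OrganPuzzleDrawer found by class lookup, so it is hard-wired to jar A.
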(event `self.ReceiveBeginPlay`
  (`SceneComponent.SetVisibility` (`self.StaticMesh`) false false))

(event `self.Box.OnComponentBeginOverlap`
  (params (OverlappedComponent :type "PrimitiveComponent Object Reference") (OtherActor :type "Actor Object Reference") (OtherComp :type "PrimitiveComponent Object Reference") (OtherBodyIndex :type Integer) (bFromSweep :type Boolean) (SweepResult :type "HitResult Structure (by ref)"))
  (if (`ActorComponent.ComponentHasTag` OtherComp (`self.Tag`))
    (`ActorComponent.K2_DestroyComponent` OtherComp)
    (`SceneComponent.SetVisibility` (`self.StaticMesh`) true false)
    (`|ExecutionSequence`
      (:`then_0`
        (bind _outactors (`GameplayStatics.GetAllActorsOfClass` "/Game/Blueprints/NamedAssets/ItemBP_Jar1_C.ItemBP_Jar1_C_C"))
        (`/Game/Blueprints/NamedAssets/ItemBP_Jar1_C.DestroyItem` _outactors))
      (:`then_1`
        (bind _returnvalue (`GameplayStatics.GetActorOfClass` "/Game/Blueprints/BP_OrganPuzzleDrawer.BP_OrganPuzzleDrawer_C"))
        (`/Game/Blueprints/BP_OrganPuzzleDrawer.SetValJarA` _returnvalue)))))

(fn `UserConstructionScript`)