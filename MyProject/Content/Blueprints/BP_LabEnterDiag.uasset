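; A one-shot trigger that plays a dialogue line when the player enters an area, likely the lab.
; When BP_FirstPersonCharacter overlaps its box, a DoOnce gate plays a 2D voice clip and shows the WB_Dialogue5 widget in the viewport.
; After a short delay, it removes the widget if it is still valid.
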(event `self.Box.OnComponentBeginOverlap`
  (params (OverlappedComponent :type "PrimitiveComponent Object Reference") (OtherActor :type "Actor Object Reference") (OtherComp :type "PrimitiveComponent Object Reference") (OtherBodyIndex :type Integer) (bFromSweep :type Boolean) (SweepResult :type "HitResult Structure (by ref)"))
  (bind _diag5 (`self.Diag5`))
  (cast `/Game/FirstPerson/Blueprints/BP_FirstPersonCharacter` OtherActor)
  (`/Engine/EditorBlueprintResources/StandardMacros.DoOnce` false
    (:`Completed`
      (`|ExecutionSequence`
        (:`then_0`
          (`GameplayStatics.PlaySound2D` "/Game/Sounds/FinalVoiceLines/6__Now_What_Do_We_Have_In_Here.6__Now_What_Do_We_Have_In_Here" 1.0 1.0 0.0 null null))
        (:`then_1`
          (bind _returnvalue (`|CreateWidget` "/Game/Blueprints/UI/Dialogue/WB_Dialogue5.WB_Dialogue5_C"))
          (bind _output_get (set `self.Diag5` _returnvalue))
          (`UserWidget.AddToViewport` _output_get 0)
          (`KismetSystemLibrary.Delay` 3.5)
          (`/Engine/EditorBlueprintResources/StandardMacros.IsValid` _diag5
            (:`Is Valid`
              (`Widget.RemoveFromParent` _diag5))))))))

(fn `UserConstructionScript`)